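; Player controller that turns Enhanced Input into movement, mouse look and jump on the BP_Player character.
; On BeginPlay it adds the IMC_Main mapping context and caches the BP_Player found with GetActorOfClass, rather than using the possessed pawn.
; Move, look and jump input actions forward their values to that character's Move, MouseLook and Jump functions, so the character owns the actual movement logic.
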(event `self.ReceiveBeginPlay`
  (`EnhancedInputSubsystemInterface.AddMappingContext` (subsystem `EnhancedInputLocalPlayerSubsystem`) "/Game/Blueprints/Player/Input/IMC_Main.IMC_Main" 0 (struct))
  (bind _returnvalue (`GameplayStatics.GetActorOfClass` "/Game/Blueprints/Player/BP_Player.BP_Player_C"))
  (set `self.PlayerChar` _returnvalue))

(event `EnhancedInput|/Game/Blueprints/Player/Input/IA_Move`
  (params (ActionValue :type "Vector2D Structure") (ElapsedSeconds :type "Float (double-precision)") (TriggeredSeconds :type "Float (double-precision)") (InputAction :type "InputAction Object Reference" :default "/Game/Blueprints/Player/Input/IA_Move.IA_Move"))
  (:`Triggered`
    (`PlayerChar.Move` (`self.PlayerChar`) ActionValue_X ActionValue_Y)))

(event `EnhancedInput|/Game/Blueprints/Player/Input/IA_MouseLook`
  (params (ActionValue :type "Vector2D Structure") (ElapsedSeconds :type "Float (double-precision)") (TriggeredSeconds :type "Float (double-precision)") (InputAction :type "InputAction Object Reference" :default "/Game/Blueprints/Player/Input/IA_MouseLook.IA_MouseLook"))
  (:`Triggered`
    (`PlayerChar.MouseLook` (`self.PlayerChar`) ActionValue_X ActionValue_Y)))

(event `EnhancedInput|/Game/Blueprints/Player/Input/IA_Jump`
  (params (ActionValue :type Boolean) (ElapsedSeconds :type "Float (double-precision)") (TriggeredSeconds :type "Float (double-precision)") (InputAction :type "InputAction Object Reference" :default "/Game/Blueprints/Player/Input/IA_Jump.IA_Jump"))
  (:`Started`
    (`Character.Jump` (`self.PlayerChar`))))

(fn `UserConstructionScript`)