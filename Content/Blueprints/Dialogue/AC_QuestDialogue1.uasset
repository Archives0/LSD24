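; Quest dialogue component that shows either intro or completion text in a UI_DialogueBox and fires give-quest or quest-complete dispatchers when it ends.
; Text comes from maps keyed by the LSD game instance's StoryStage, with separate sets once Spoken is true, a flag both branches share.
; InitiateDialogue branches on HasQuestItem, whose inventory check is left unconnected.
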(event `self.ReceiveBeginPlay`
  (bind _aslsd (cast `LSD` (`GameplayStatics.GetGameInstance`)))
  (set `self.LSD` _aslsd))

(event `InitiateDialogue`
  (if (`self.HasQuestItem`)
    (`self.CompletedDialogue`)
    (else
      (`self.IntroDialogue`))))

(event `IntroDialogue`
  (bind _returnvalue (`|CreateWidget` "/Game/Blueprints/UI/Widgets/UI_DialogueBox.UI_DialogueBox_C" null (`self.GetTextBlock`) (/ 1 (`self.TextSpeed`))))
  (`UserWidget.AddToViewport` _returnvalue 0)
  (add `/Game/Blueprints/UI/Widgets/UI_DialogueBox.OnDialogueEnd` _returnvalue (delegate `IntroEnd`))
  (set `self.Spoken` true))

(event `IntroEnd`
  (`self.OnGiveQuest`))

(event `CompletedDialogue`
  (bind _returnvalue (`|CreateWidget` "/Game/Blueprints/UI/Widgets/UI_DialogueBox.UI_DialogueBox_C" null (`self.GetCompletedText`) (/ 1 (`self.TextSpeed`))))
  (`UserWidget.AddToViewport` _returnvalue 0)
  (add `/Game/Blueprints/UI/Widgets/UI_DialogueBox.OnDialogueEnd` _returnvalue (delegate `CompletedEnd`))
  (set `self.Spoken` true))

(event `CompletedEnd`
  (`self.OnQuestComplete`))

(fn `GetCompletedText`
  (returns (Text :type "Array of String"))
  (bind (_value _returnvalue) (`BlueprintMapLibrary.Map_Find` (`self.QuestCompleteText`) (`LSD.storyStage` (`self.LSD`))))
  (bind (_value_2 _returnvalue_2) (`BlueprintMapLibrary.Map_Find` (`self.SpokenCompleteText`) (`LSD.storyStage` (`self.LSD`))))
  (if (`self.Spoken`)
    (if _returnvalue_2
      (set `self.CurrentTXT` (`.textOptions` (break `Dialogue` _value_2)))
      (return (`self.CurrentTXT`))
      (else
        _))
    (elif _returnvalue
      (set `self.CurrentTXT` (`.textOptions` (break `Dialogue` _value)))
      (return (`self.CurrentTXT`))
      (else
        _)))
  (`KismetSystemLibrary.PrintString` "No dialogue found at game stage."))

(fn `GetTextBlock`
  (returns (Text :type "Array of String"))
  (bind (_value _returnvalue) (`BlueprintMapLibrary.Map_Find` (`self.DialogueText`) (`LSD.storyStage` (`self.LSD`))))
  (bind (_value_2 _returnvalue_2) (`BlueprintMapLibrary.Map_Find` (`self.SpokenDialogueText`) (`LSD.storyStage` (`self.LSD`))))
  (if (`self.Spoken`)
    (if _returnvalue_2
      (set `self.CurrentTXT` (`.textOptions` (break `Dialogue` _value_2)))
      (return (`self.CurrentTXT`))
      (else
        _))
    (elif _returnvalue
      (set `self.CurrentTXT` (`.textOptions` (break `Dialogue` _value)))
      (return (`self.CurrentTXT`))
      (else
        _)))
  (`KismetSystemLibrary.PrintString` "No dialogue found at game stage."))