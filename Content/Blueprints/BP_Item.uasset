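; BP_Item is an interactable pickup that adds its item to the player's inventory.
; It caches the LSD game instance on BeginPlay, and its Interaction event passes the Item to that instance's AddToInventory.
; It then fires the OnPickedUp dispatcher, hides its component hierarchy and disables collision rather than destroying the actor.
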(event `self.ReceiveBeginPlay`
  (bind _aslsd (cast `LSD` (`GameplayStatics.GetGameInstance`)))
  (set `self.LSD` _aslsd))

(event `self.Interaction`
  (params (hit :type "HitResult Structure"))
  (`LSD.AddToInventory` (`self.LSD`) (`self.Item`))
  (`self.OnPickedUp`)
  (`SceneComponent.SetVisibility` (`self.RootComponent`) false true)
  (`self.SetActorEnableCollision` false))

(fn `UserConstructionScript`)