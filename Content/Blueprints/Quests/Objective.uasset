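; Quest objective Blueprint that tracks its own active and completed state and reports binary progress based on completion.
; Completing it sets the completed flag and calls OnObjectiveComplete, passing itself.
; It returns its ID in a list when completed, and completes itself when a supplied list contains that ID, so completion state can be collected and reapplied by ID.
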(fn `CompleteObjective`
  (set `self.Completed` true)
  (`self.OnObjectiveComplete` self))

(fn `GetCompletedObjectives`
  (returns (Objectives :type "Array of String"))
  (if (`self.Completed`)
    (return (`|MakeArray` (`self.ID`)))
    (else
      (return))))

(fn `GetProgress`
  (returns (Progress :type "Float (double-precision)"))
  (return (`KismetMathLibrary.SelectFloat` 1.0 0.0 (`self.Completed`))))

(fn `SetObjectiveComplete`
  (params (Objectives :type "Array of String"))
  (if (`KismetArrayLibrary.Array_Contains` Objectives (`self.ID`))
    (`self.CompleteObjective`)))

(fn `StartObjective`
  (set `self.Active` true))