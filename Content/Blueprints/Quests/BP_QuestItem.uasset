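; BP_QuestItem is a quest item pickup that the player collects through an Interaction event.
; BeginPlay caches the LSD game instance, which holds the PlayerItems collection.
; Interaction adds the Item to PlayerItems and calls the OnItemPickedUp dispatcher.
; It then hides the static mesh and disables its collision, leaving the actor in the level.
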(event `self.ReceiveBeginPlay`
  (bind _aslsd (cast `LSD` (`GameplayStatics.GetGameInstance`)))
  (set `self.LSD` _aslsd))

(event `self.Interaction`
  (params (hit :type "HitResult Structure"))
  (bind _staticmesh (`self.StaticMesh`))
  (`KismetArrayLibrary.Array_Add` (`LSD.playerItems` (`self.LSD`)) (`self.Item`))
  (`self.OnItemPickedUp`)
  (`SceneComponent.SetVisibility` _staticmesh false false)
  (`PrimitiveComponent.SetCollisionEnabled` _staticmesh "NoCollision"))

(fn `UserConstructionScript`)