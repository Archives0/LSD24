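; BP_FetchQuest is a quest Blueprint that asks the player to fetch a quest item.
; On StartQuest it constructs a FetchObjective for the QuestItem with test name and ID, starts it, spawns the item and binds to the objective's completion.
; When the objective completes, it broadcasts OnQuestComplete with itself and prints a completion message.
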(event `self.StartQuest`
  (bind _newparam (`self.InitializeObjectives`))
  (bind _output_get (set `self.Objective` _newparam))
  (`/Game/Blueprints/Quests/Objectives/Objective.StartObjective` _output_get)
  (`/Game/Blueprints/Quests/BP_QuestItem.SpawnItem` (`self.Quest Item`))
  (add `/Game/Blueprints/Quests/Objectives/Objective.OnObjectiveComplete` _output_get (delegate `self.QuestComplete`)))

(event `self.QuestComplete`
  (params (Objective :type "/Game/Blueprints/Quests/Objectives/Objective Object Reference"))
  (`self.OnQuestComplete` self)
  (`KismetSystemLibrary.PrintString` "Quest completed"))

(fn `InitializeObjectives`
  (returns (NewParam :type "/Game/Blueprints/Quests/Objectives/Objective Object Reference"))
  (bind _returnvalue (`|GenericCreateObject` "/Game/Blueprints/Quests/Objectives/FetchObjective.FetchObjective_C" (`self.Quest Item`) "TestItem" "TestID"))
  (return _returnvalue))

(fn `UserConstructionScript`
  (`parent.UserConstructionScript`))