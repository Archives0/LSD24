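; AC_QuestLog is a quest log component that tracks active and finished quests in two maps keyed by QuestID.
; AddQuest checks both states, then stores the quest, starts it and binds an event to its completion.
; CompleteQuest moves a quest from the active map to the finished map.
; The Contains lookups in IsQuestActive and IsQuestFinished appear unconnected, and BeginPlay and Tick are empty.
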(fn `AddQuest`
  (params (NewQuest :type "/Game/Blueprints/Quests/BP_Quest Object Reference"))
  (bind _newquest (`local.NewQuest`))
  (if (and (== (`self.IsQuestActive` NewQuest) false) (== (`self.IsQuestFinished` NewQuest) false))
    (`BlueprintMapLibrary.Map_Add` (`self.ActiveQuests`) (`/Game/Blueprints/Quests/BP_Quest.QuestID` _newquest) _newquest)
    (`/Game/Blueprints/Quests/BP_Quest.StartQuest` _newquest)
    (add `/Game/Blueprints/Quests/BP_Quest.OnQuestComplete` _newquest (`|CreateDelegate` :!event `CompleteQuest`))))

(fn `CompleteQuest`
  (params (Quest :type "/Game/Blueprints/Quests/BP_Quest Object Reference"))
  (bind _questid (`/Game/Blueprints/Quests/BP_Quest.QuestID` Quest))
  (`BlueprintMapLibrary.Map_Remove` (`self.ActiveQuests`) _questid)
  (`BlueprintMapLibrary.Map_Add` (`self.FinishedQuests`) _questid (`local.Quest`)))