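; BP_RotDoor is an interactable door actor that toggles between open and closed by rotating.
; On Interaction, the Open or Close timeline plays from the start, lerping the whole actor's rotation between StartRot and EndRot.
; A Moving flag ignores interactions mid-swing, and Opened records the state when each timeline finishes.
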(event `self.Interaction`
  (params (hit :type "HitResult Structure"))
  (if (`self.Moving`)
    _
    (elif (`self.Opened`)
      (set `self.Moving` true)
      (bind (_direction _alpha) (`Timeline|Close` :!via `PlayFromStart`)
        (:`Update`
          (`self.K2_SetActorRotation` (`KismetMathLibrary.RLerp` (`self.EndRot`) (`self.StartRot`) _alpha)))
        (:`Finished`
          (set `self.Opened` false)
          (set `self.Moving` false)))
      (else
        (set `self.Moving` true)
        (bind (_direction_2 _alpha_2) (`Timeline|Open` :!via `PlayFromStart`)
          (:`Update`
            (`self.K2_SetActorRotation` (`KismetMathLibrary.RLerp` (`self.StartRot`) (`self.EndRot`) _alpha_2)))
          (:`Finished`
            (set `self.Opened` true)
            (set `self.Moving` false)))))))

(fn `UserConstructionScript`)