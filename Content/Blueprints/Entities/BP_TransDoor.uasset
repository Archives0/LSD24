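; BP_TransDoor is a sliding door actor that toggles between open and closed on its Interaction event.
; Open and Close timelines drive SetActorLocation, with Opened tracking state and Moving blocking interaction mid-motion.
; Opening lerps StartPos to EndPos, but closing has a fixed zero alpha, so it holds at EndPos while still marking itself closed.
; The construction script applies the configurable Mesh.
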(event `self.Interaction`
  (params (hit :type "HitResult Structure"))
  (if (`self.Moving`)
    _
    (elif (`self.Opened`)
      (set `self.Moving` true)
      (`Timeline|Close` :!via `PlayFromStart`
        (:`Update`
          (`self.K2_SetActorLocation` (`KismetMathLibrary.VLerp` (`self.EndPos`) (`self.StartPos`))))
        (:`Finished`
          (set `self.Opened` false)
          (set `self.Moving` false)))
      (else
        (set `self.Moving` true)
        (bind (_direction _alpha) (`Timeline|Open` :!via `PlayFromStart`)
          (:`Update`
            (`self.K2_SetActorLocation` (`KismetMathLibrary.VLerp` (`self.StartPos`) (`self.EndPos`) _alpha)))
          (:`Finished`
            (set `self.Opened` true)
            (set `self.Moving` false)))))))

(fn `UserConstructionScript`
  (`StaticMeshComponent.SetStaticMesh` (`self.StaticMesh`) (`self.Mesh`)))