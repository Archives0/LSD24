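; BP_QuestGiver is an interactable entity that hands the player a quest and closes it out once its conditions are met.
; On interaction, its ACQuestDialogue component plays intro or completed dialogue depending on the QuestComplete flag.
; Dialogue events add or complete the Quest in the player pawn's AC_QuestLog.
; The Quest's own completion event sets the flag and resets the dialogue's Spoken state.
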(event `self.Interaction`
  (params (hit :type "HitResult Structure"))
  (bind _ac_questdialogue (`self.AC_QuestDialogue`))
  (if (`self.QuestComplete`)
    (`/Game/Blueprints/Dialogue/AC_QuestDialogue.CompletedDialogue` _ac_questdialogue)
    (else
      (`/Game/Blueprints/Dialogue/AC_QuestDialogue.IntroDialogue` _ac_questdialogue))))

(event `self.ReceiveBeginPlay`
  (bind _ac_questdialogue (`self.AC_QuestDialogue`))
  (add `/Game/Blueprints/Dialogue/AC_QuestDialogue.OnGiveQuest` _ac_questdialogue (delegate `GiveQuest`))
  (add `/Game/Blueprints/Quests/BP_Quest.OnQuestComplete` (`self.Quest`) (delegate `ConditionMet`))
  (add `/Game/Blueprints/Dialogue/AC_QuestDialogue.OnQuestComplete` _ac_questdialogue (delegate `CompleteQuest`)))

(event `GiveQuest`
  (`/Game/Blueprints/Quests/AC_QuestLog.AddQuest` (`self.GetComponentByClass` (`GameplayStatics.GetPlayerPawn` 0) "/Game/Blueprints/Quests/AC_QuestLog.AC_QuestLog_C") (`self.Quest`)))

(event `CompleteQuest`
  (`/Game/Blueprints/Quests/AC_QuestLog.CompleteQuest` (`self.GetComponentByClass` (`GameplayStatics.GetPlayerPawn` 0) "/Game/Blueprints/Quests/AC_QuestLog.AC_QuestLog_C") (`self.Quest`)))

(event `ConditionMet`
  (params (Quest :type "/Game/Blueprints/Quests/BP_Quest Object Reference"))
  (set `self.QuestComplete` true)
  (set `/Game/Blueprints/Dialogue/AC_QuestDialogue.Spoken` false (`self.AC_QuestDialogue`)))

(fn `UserConstructionScript`)